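; BP_lampe is a lamp actor whose spotlight the player toggles with F.
; Entering its box enables input on the lamp and toggles the prompt's visibility.
; Leaving toggles the prompt again and calls DisableInput on the player controller itself, not on the lamp.
; The construction script applies a configurable light color and initial visibility to the spotlight.
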(event OnComponentBeginOverlap(Box)
  (params (OverlappedComponent :type Primitive%20Component%20Object%20Reference) (OtherActor :type Actor%20Object%20Reference) (OtherComp :type Primitive%20Component%20Object%20Reference) (OtherBodyIndex :type Integer) (bFromSweep :type Boolean) (SweepResult :type Hit%20Result%20Structure%20%28by%20ref%29))
  (Input|EnableInput (Game|GetPlayerController 0))
  (Rendering|ToggleVisibility (Variables|Default|Getpromt) false))

(event OnComponentEndOverlap(Box)
  (params (OverlappedComponent :type Primitive%20Component%20Object%20Reference) (OtherActor :type Actor%20Object%20Reference) (OtherComp :type Primitive%20Component%20Object%20Reference) (OtherBodyIndex :type Integer))
  (Input|DisableInput (Game|GetPlayerController 0) 0)
  (Rendering|ToggleVisibility (Variables|Default|Getpromt) false))

(event Input|KeyboardEvents|F
  (params (Key :type Key%20Structure :default "None"))
  (:Pressed
    (Rendering|ToggleVisibility (Variables|Default|GetSpotLight) false)))

(fn ConstructionScript
  (bind _spotlight (Variables|Default|GetSpotLight))
  (Rendering|Components|Light|SetLightColor _spotlight (Variables|Default|GetNew%20Light%20Color) true)
  (Rendering|SetVisibility _spotlight (Variables|Default|GetNew%20Visibility) false))